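; BP_Button is an interactable button that starts targets sharing its value.
; Overlapping its sphere shows a widget, and leaving hides it.
; Interact plays a sound, then searches all BP_Target actors and calls StartTarget with the interactor on those whose TargetValue matches ButtonValue.
; A camera view-target blend and a return value in Interact are left unconnected.
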(event `self.Sphere.OnComponentBeginOverlap`
  (params (OverlappedComponent :type "PrimitiveComponent Object Reference") (OtherActor :type "Actor Object Reference") (OtherComp :type "PrimitiveComponent Object Reference") (OtherBodyIndex :type Integer) (bFromSweep :type Boolean) (SweepResult :type "HitResult Structure (by ref)"))
  (`SceneComponent.SetHiddenInGame` (`self.Widget`) false false))

(event `self.Sphere.OnComponentEndOverlap`
  (params (OverlappedComponent :type "PrimitiveComponent Object Reference") (OtherActor :type "Actor Object Reference") (OtherComp :type "PrimitiveComponent Object Reference") (OtherBodyIndex :type Integer))
  (`SceneComponent.SetHiddenInGame` (`self.Widget`) true false))

(fn `Interact`
  (params (Interactor :type "Character Object Reference"))
  (returns (`DidInteract?` :type Boolean))
  (locals (NewLocalVar_0 :type Boolean :default true))
  (`GameplayStatics.SpawnSound2D` "/Game/Audio/Music/Background_Music/background_music_2.background_music_2" 1.0 1.0 0.0 null)
  (bind _outactors (`GameplayStatics.GetAllActorsOfClass` "/Game/Blueprints/BP_Target.BP_Target_C"))
  (for _array_element _outactors
    (if (== (`/Game/Blueprints/BP_Target.TargetValue` _array_element) (`self.ButtonValue`))
      (`/Game/Blueprints/BP_Target.StartTarget` _array_element Interactor))))

(fn `UserConstructionScript`)