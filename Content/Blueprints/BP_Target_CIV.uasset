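; BP_Target_CIV is a shooting-range target, apparently a civilian, that penalizes the player's score when shot.
; StartTarget swings the Cube from lying flat to upright on a timeline, then after a short delay returns the view target to the given Player.
; A hit from a first-person projectile subtracts points from the character's Score and plays a second timeline that folds the Cube back down.
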(event `StartTarget`
  (params (Player :type "Actor Object Reference"))
  (bind (_direction _start) (`Timeline|Timeline_0`)
    (:`Update`
      (`SceneComponent.K2_SetRelativeRotation` (`self.Cube`) (`KismetMathLibrary.RLerp` (struct :`Roll` -90.0) (struct) _start) false false))
    (:`Finished`
      (`KismetSystemLibrary.Delay` 1.0)
      (`PlayerController.SetViewTargetWithBlend` (`GameplayStatics.GetPlayerController` 0) Player 0.0 "VTBlend_Linear" 0.0 false))))

(event `self.ReceiveHit`
  (params (MyComp :type "PrimitiveComponent Object Reference") (Other :type "Actor Object Reference") (OtherComp :type "PrimitiveComponent Object Reference") (bSelfMoved :type Boolean) (HitLocation :type "Vector Structure") (HitNormal :type "Vector Structure") (NormalImpulse :type "Vector Structure") (Hit :type "HitResult Structure (by ref)"))
  (bind _as_bp_first_person_character (`self.As BP First Person Character`))
  (cast `/Game/FirstPerson/Blueprints/BP_FirstPersonProjectile` Other)
  (bind _asbp_first_person_character (cast `/Game/FirstPerson/Blueprints/BP_FirstPersonCharacter` (`GameplayStatics.GetPlayerCharacter` 0)))
  (set `self.As BP First Person Character` _asbp_first_person_character)
  (set `/Game/FirstPerson/Blueprints/BP_FirstPersonCharacter.Score` (- (`/Game/FirstPerson/Blueprints/BP_FirstPersonCharacter.Score` _as_bp_first_person_character) 5) _as_bp_first_person_character)
  (bind (_direction _down) (`Timeline|Timeline_1`)
    (:`Update`
      (`SceneComponent.K2_SetRelativeRotation` (`self.Cube`) (`KismetMathLibrary.RLerp` (struct) (struct :`Roll` -90.0) _down) false false))))

(fn `UserConstructionScript`)